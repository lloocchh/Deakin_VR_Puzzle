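; Physics ball actor that replaces itself with a new ball on overlapping the reset sheet or after a 10-second delay.
; Respawning detaches the trail, drops the sphere out of sight, gives the actor a short lifespan and spawns a successor at StartLocation.
; Overlaps also scale velocity on the blue panel and play a throttled bounce sound.
; Tick moves StartLocation for levels 2 and 3 based on player X position.
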(event EventBeginPlay
  (Variables|Default|SetStart%20Location (Variables|/Script/Engine.SceneComponent|GetRelativeLocation (Variables|Default|GetSphere)))
  (Utilities|FlowControl|RetriggerableDelay 1e+01 :!label _label)
  ;[1 1 1] Hide Collided Ball
  (Transformation|DetachFromComponent (Variables|Default|GetMS_BallTrail) "KeepWorld" "KeepWorld" "KeepWorld" true)
  (Transformation|SetRelativeLocationAndRotation (Variables|Default|GetSphere) "0.000000,0.000000,-1100.000000" "0, 0, 0" false true)
  (Actor|SetLifeSpan 4.0)
  ;[1 1 1] Spawn New Ball
  (Game|SpawnActorfromClass "BP_Ball_C" (Math|Conversions|ToTransform(Vector) (Variables|Default|GetStart%20Location)) "AlwaysSpawn" "MultiplyWithRoot" 0 (Variables|Default|GetBallResetSheet) (Variables|Default|GetBlue_Panel) 0)
  (goto _label))

(event EventTick
  (params (DeltaSeconds :type Float%20%28single-precision%29))
  (bind _returnvalue (Game|Player|GetPlayerPawn 0))
  (bind _returnvalue_2 (Transformation|GetActorLocation _returnvalue))
  ;[1 1 1] Update Ball Spawn Location For Next Level
  (if (and (< (.x _returnvalue_2) 7.5e+02) (> (.x _returnvalue_2) -2.5e+02))
    (Utilities|FlowControl|DoOnce false)
    (elif (and (< (.x _returnvalue_2) -2.5e+02) (> (.x _returnvalue_2) -1.25e+03))
      (Utilities|FlowControl|DoOnce false
        (:Completed
          (Variables|Default|SetStart%20Location "-850.000000,50.000000,350.000000")))
      (elif (and (< (.x _returnvalue_2) -1.25e+03) (> (.x _returnvalue_2) -2.25e+03))
        (Utilities|FlowControl|DoOnce false
          (:Completed
            (Variables|Default|SetStart%20Location "-1850.000000,50.000000,350.000000")))))))

(event Collision|EventActorBeginOverlap
  (params (OtherActor :type Actor%20Object%20Reference))
  ;[1 1 1] Reset Ball On Collision With Reset Sheet
  (if (== OtherActor (Variables|Default|GetBallResetSheet))
    ;[1 1 1] Hide Collided Ball
    (Transformation|DetachFromComponent (Variables|Default|GetMS_BallTrail) "KeepWorld" "KeepWorld" "KeepWorld" true :!label _label)
    (Transformation|SetRelativeLocationAndRotation (Variables|Default|GetSphere) "0.000000,0.000000,-1100.000000" "0, 0, 0" false true)
    (Actor|SetLifeSpan 4.0)
    ;[1 1 1] Spawn New Ball
    (Game|SpawnActorfromClass "BP_Ball_C" (Math|Conversions|ToTransform(Vector) (Variables|Default|GetStart%20Location)) "AlwaysSpawn" "MultiplyWithRoot" 0 (Variables|Default|GetBallResetSheet) (Variables|Default|GetBlue_Panel) 0)
    (Utilities|FlowControl|RetriggerableDelay 1e+01)
    (goto _label)
    (else
      (Utilities|FlowControl|Sequence
        (:then_0
          ;[1 1 1] Blue Panel Speed Boost
          (if (== OtherActor (Variables|Default|GetBlue_Panel))
            (Physics|SetPhysicsLinearVelocity (Variables|Default|GetSphere) (* (Transformation|GetComponentVelocity (Variables|Default|GetSphere)) (Variables|Default|GetBlue_Panel_Modifer)) false "None")))
        (:then_1
          ;[1 1 1] Ball Bounce Sound
          (Utilities|FlowControl|DoOnce false :!label _label_2
            (:Completed
              (Audio|PlaySound2D "/Game/Audio/BallBounceSoundCue.BallBounceSoundCue" 1.0 1.0 0.0 0 0)
              (Utilities|FlowControl|Delay 0.15)
              (goto _label_2 Reset))))))))

(fn ConstructionScript)